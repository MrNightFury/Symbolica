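; Teaser character with colored spell effects on both arms, a fireball cast, and a title widget shown on BeginPlay.
; Construction tints both spells and builds a ring of small point lights around each.
; Tick spins the right ring (the left's rotation is zero) and feeds the Target position to the right-arm effect.
; StartFireball enables that effect's Collection emitter, then after delays ramps the fireball light and triggers its audio and Niagara effect.
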(event `self.ReceiveTick`
  (params (DeltaSeconds :type "Float (single-precision)"))
  (bind _rightarmspell (`self.RightArmSpell`))
  (bind _returnvalue (`SceneComponent.K2_GetComponentLocation` (`self.Target`)))
  (`|ExecutionSequence`
    (:`then_0`
      (for _array_element (`self.RightLights`)
        (`SceneComponent.K2_SetRelativeLocation` _array_element (`KismetMathLibrary.GreaterGreater_VectorRotator` (`SceneComponent.RelativeLocation` _array_element) (`KismetMathLibrary.MakeRotator` 0.0 0.0 (* DeltaSeconds -45.0))) false false)))
    (:`then_1`
      (for _array_element_2 (`self.LeftLights`)
        (`SceneComponent.K2_SetRelativeLocation` _array_element_2 (`KismetMathLibrary.GreaterGreater_VectorRotator` (`SceneComponent.RelativeLocation` _array_element_2) (`KismetMathLibrary.MakeRotator` 0.0 0.0 (* 0.0 -45.0))) false false)))
    (:`then_2`
      (`FXSystemComponent.SetVectorParameter` _rightarmspell "TargetPosition" (- _returnvalue (`SceneComponent.K2_GetComponentLocation` (`self.RightArmSpell`))))
      (`NiagaraComponent.SetVariablePosition` _rightarmspell "TargetPositionAbsolute" _returnvalue))))

(event `StartFireball`
  (bind _a_fireball_cue (`self.A_Fireball_Cue`))
  (`FXSystemComponent.SetEmitterEnable` (`self.RightArmSpell`) "Collection" true)
  (`KismetSystemLibrary.Delay` 0.25)
  (`|ExecutionSequence`
    (:`then_0`
      (bind (_direction _scale) (`Timeline|Timeline`)
        (:`Update`
          (`LightComponent.SetIntensity` (`self.FireballLight`) (* _scale 100.0)))))
    (:`then_1`
      (`AudioComponent.FadeIn` _a_fireball_cue 0.0 1.0 0.0 "Linear")
      (`KismetSystemLibrary.Delay` 0.25)
      (`ActorComponent.Activate` _a_fireball_cue false)
      (`ActorComponent.Activate` (`self.NS_Fireball`) false))))

(event `self.ReceiveBeginPlay`
  (`FXSystemComponent.SetEmitterEnable` (`self.RightArmSpell`) "Collection" false)
  (bind _returnvalue (`|CreateWidget` "/Game/Teaser/WBP_Title.WBP_Title_C" (`GameplayStatics.GetPlayerController` 0)))
  (`UserWidget.AddToViewport` _returnvalue 0))

(fn `UserConstructionScript`
  (bind _rightcolor (`self.RightColor`))
  (bind _leftcolor (`self.LeftColor`))
  (`FXSystemComponent.SetColorParameter` (`self.RightArmSpell`) "MainColor" _rightcolor)
  (`LightComponent.SetLightColor` (`self.RightArmSpellLight`) _rightcolor true)
  (`FXSystemComponent.SetColorParameter` (`self.LeftArmSpell`) "MainColor" _leftcolor)
  (`LightComponent.SetLightColor` (`self.LeftArmSpellLight`) _leftcolor true)
  (`FXSystemComponent.SetVectorParameter` (`self.RightArmSpell`) "TargetPosition" (`SceneComponent.RelativeLocation` (`self.SpringArm`)))
  (`|ExecutionSequence`
    (:`then_0`
      (for _index (range 10)
        (bind _returnvalue (`AddComponent|NODE_AddPointLightComponent-0` :`bManualAttachment` true))
        (`SceneComponent.K2_AttachToComponent` _returnvalue (`self.RightArmSpell`) "None" "KeepRelative" "KeepRelative" "KeepRelative" true)
        (`LightComponent.SetIntensity` _returnvalue 0.5)
        (`SceneComponent.K2_SetRelativeLocation` _returnvalue (`KismetMathLibrary.GreaterGreater_VectorRotator` (`KismetMathLibrary.MakeVector` 0.0 20.0) (`KismetMathLibrary.MakeRotator` 0.0 0.0 (* 36.0 _index))) false false)
        (`LightComponent.SetLightColor` _returnvalue (`self.RightColor`) true)
        (`LocalLightComponent.SetAttenuationRadius` _returnvalue 20.0)
        (`KismetArrayLibrary.Array_Add` (`self.RightLights`) _returnvalue)))
    (:`then_1`
      (for _index_2 (range 10)
        (bind _returnvalue_2 (`AddComponent|NODE_AddPointLightComponent-1` :`bManualAttachment` true))
        (`SceneComponent.K2_AttachToComponent` _returnvalue_2 (`self.LeftArmSpell`) "None" "KeepRelative" "KeepRelative" "KeepRelative" true)
        (`LightComponent.SetIntensity` _returnvalue_2 0.5)
        (`SceneComponent.K2_SetRelativeLocation` _returnvalue_2 (`KismetMathLibrary.GreaterGreater_VectorRotator` (`KismetMathLibrary.MakeVector` 0.0 20.0) (`KismetMathLibrary.MakeRotator` 0.0 0.0 (* 36.0 _index_2))) false false)
        (`LightComponent.SetLightColor` _returnvalue_2 (`self.LeftColor`) true)
        (`LocalLightComponent.SetAttenuationRadius` _returnvalue_2 20.0)
        (`KismetArrayLibrary.Array_Add` (`self.LeftLights`) _returnvalue_2)))))