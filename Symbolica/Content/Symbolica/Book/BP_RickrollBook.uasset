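; BP_RickrollBook is a grabbable book that opens when held and plays media as a rickroll gag.
; Grab and drop events from BP_GrabComponent open and close the book, notify its WBP_Book widget, and start or stop MediaSound at reduced volume.
; One BookMesh animation serves both directions: BeginPlay seeks to a preset position, then a negative play rate opens it and a positive one closes it.
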(event `self.ReceiveBeginPlay`
  (`SkeletalMeshComponent.SetPosition` (`self.BookMesh`) 2.5 true))

(event `SetOpened`
  (params (bIsOpen :type Boolean))
  (bind _bookmesh (`self.BookMesh`))
  (if bIsOpen
    (`SkeletalMeshComponent.SetPlayRate` _bookmesh -5.0)
    (else
      (`SkeletalMeshComponent.SetPlayRate` _bookmesh 5.0)))
  (`SkeletalMeshComponent.Play` _bookmesh false))

(event `self.BP_GrabComponent.OnGrabbed`
  (bind _mediasound (`self.MediaSound`))
  (`self.SetOpened` true)
  (bind _aswbp_book (cast `/Game/Symbolica/Core/Book/WBP_Book` (`WidgetComponent.GetWidget` (`self.Widget`))))
  (`/Game/Symbolica/Core/Book/WBP_Book.OnOpen` _aswbp_book)
  (`SynthComponent.Start` _mediasound)
  (`SynthComponent.SetVolumeMultiplier` _mediasound 0.25))

(event `self.BP_GrabComponent.OnDropped`
  (`self.SetOpened` false)
  (bind _aswbp_book (cast `/Game/Symbolica/Core/Book/WBP_Book` (`WidgetComponent.GetWidget` (`self.Widget`))))
  (`/Game/Symbolica/Core/Book/WBP_Book.OnClose` _aswbp_book)
  (`SynthComponent.Stop` (`self.MediaSound`)))

(fn `UserConstructionScript`)