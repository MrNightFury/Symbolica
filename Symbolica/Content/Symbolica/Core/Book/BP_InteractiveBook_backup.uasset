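; VR spellbook menu actor that opens when grabbed, closes on drop and can glide back to its Origin.
; UpdatePageSequence builds title, symbol, spell and settings sections from widgets and DataTable row counts, plus bookmarks.
; BPBookSequenceManager drives page setups, which BPWidgetsManager shows on left and right panels.
; While held, the free hand's widget interactor clicks pages and flips them through timed, angle-checked swipes near FlipPivot.
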(event `self.ReceiveBeginPlay`
  (bind _bp_widgetsmanager (`self.BP_WidgetsManager`))
  (`|ExecutionSequence`
    (:`then_0`
      (`/Game/Symbolica/Core/MultiWidgetMenu/BP_WidgetsManager.AddPanel` _bp_widgetsmanager "Left" (`self.LeftpageWidget`) 0)
      (`/Game/Symbolica/Core/MultiWidgetMenu/BP_WidgetsManager.AddPanel` _bp_widgetsmanager "Right" (`self.RightPageWidget`) 1)
      (`self.UpdatePageSequence`))
    (:`then_1`
      (`SkeletalMeshComponent.SetPosition` (`self.BookMesh`) 2.5 true)
      (`self.UpdatePageSequence`)
      (`/Game/Symbolica/Core/MultiWidgetMenu/BP_BookSequenceManager.SetPage` (`self.BP_BookSequenceManager`) 0)
      (`self.K2_AttachToComponent` (`self.Origin`) "None" "KeepWorld" "KeepWorld" "KeepWorld" false))))

(event `Open`
  (`self.SetOpened` true))

(event `SetOpened`
  (params (bIsOpen :type Boolean))
  (bind _bookmesh (`self.BookMesh`))
  (bind _bp_widgetsmanager (`self.BP_WidgetsManager`))
  (if bIsOpen
    (`SkeletalMeshComponent.SetPlayRate` _bookmesh -5.0)
    (`/Game/Symbolica/Core/MultiWidgetMenu/BP_WidgetsManager.TransmitInteraction` _bp_widgetsmanager "NewEnumerator2" "Close")
    (else
      (`SkeletalMeshComponent.SetPlayRate` _bookmesh 5.0)
      (`/Game/Symbolica/Core/MultiWidgetMenu/BP_WidgetsManager.TransmitInteraction` _bp_widgetsmanager "NewEnumerator1" "Open")))
  (`SkeletalMeshComponent.Play` _bookmesh false))

(event `self.RightHandGrab.OnGrabbed`
  (`self.OffsetFlipPivot` false 3.0)
  (`self.SetOpened` true :!label _label)
  (`self.StopReturn`)
  (`self.UpdateControls` :!label _label_2))

(event `self.LeftHandGrab.OnGrabbed`
  (`self.OffsetFlipPivot` true 3.0)
  (goto _label))

(event `self.RightHandGrab.OnDropped`
  (`self.SetOpened` false :!label _label_3)
  (set `self.bIsReturned` false)
  (goto _label_2))

(event `Next`
  (`/Game/Symbolica/Core/MultiWidgetMenu/BP_BookSequenceManager.Next` (`self.BP_BookSequenceManager`)))

(event `self.LeftHandGrab.OnDropped`
  (goto _label_3))

(event `Prev`
  (`/Game/Symbolica/Core/MultiWidgetMenu/BP_BookSequenceManager.Prev` (`self.BP_BookSequenceManager`)))

(event `self.BP_BookSequenceManager.CurrentSetupChanged`
  (params (NewIndex :type Integer) (NewWidgets :type "/Game/Symbolica/Core/MultiWidgetMenu/S_MultiPanelWidgetSetup Structure"))
  (`/Game/Symbolica/Core/MultiWidgetMenu/BP_WidgetsManager.OpenMenuFromArray` (`self.BP_WidgetsManager`) (`.PanelsWidgets_3_354D3D7D4DC23264EA28D7B91B63AA73` (break `/Game/Symbolica/Core/MultiWidgetMenu/S_MultiPanelWidgetSetup` NewWidgets))))

(event `self.ReceiveTick`
  (params (DeltaSeconds :type "Float (single-precision)"))
  (bind _returnvalue (`self.GetActorRightVector`))
  (bind _widgetinteractor (`self.WidgetInteractor`))
  (bind _widgetinteractor_2 (`self.WidgetInteractor`))
  (bind _returnvalue_2 (`SceneComponent.K2_GetComponentLocation` (`self.WidgetInteractor`)))
  (bind (_returnvalue_bblockinghit _returnvalue_binitialoverlap _returnvalue_time _returnvalue_distance _returnvalue_location) (`GameplayStatics.BreakHitResult` (`WidgetInteractionComponent.GetLastHitResult` _widgetinteractor_2)))
  (bind _returnvalue_3 (- (`KismetSystemLibrary.GetGameTimeInSeconds`) (`self.InitialPageFlipTime`)))
  (bind _bis (`/Game/Symbolica/Core/BPFL_Utils.bIsCodirectional` (`SceneComponent.GetForwardVector` _widgetinteractor) (`self.GetActorForwardVector`) 45.0))
  (bind (_angle _bisvalid) (`/Game/Symbolica/Core/BPFL_Utils.GetAngleBetweenVectorsDegrees` (- _returnvalue_2 (`self.InitialPageFlipPosition`)) _returnvalue))
  (bind _returnvalue_4 (and _bis (< _returnvalue_3 0.5)))
  (if (`self.GetGrabbedBy`)
    (set `self.InteractorTickOffset` (- (`SceneComponent.K2_GetComponentLocation` (`self.WidgetInteractor`)) (`self.LastInteractorPosition`)))
    (`|ExecutionSequence`
      (:`then_0`
        (`self.OffsetInteractor` :!enabledstate Disabled)
        (bind _output_get (set `self.IsHoveringWidget` (and (`WidgetInteractionComponent.IsOverHitTestVisibleWidget` _widgetinteractor_2) (<= (`KismetMathLibrary.Vector_Distance` _returnvalue_location (`SceneComponent.K2_GetComponentLocation` (`self.WidgetInteractor`))) (+ (`self.InteractionOffsetValue`) (`self.AcceptableError`))))))
        (if _output_get
          (`SceneComponent.K2_SetWorldLocation` (`self.Cursor`) _returnvalue_location false false)))
      (:`then_1`
        (if true
          (if (and _bis (< (`KismetMathLibrary.VSize` (- (`SceneComponent.K2_GetComponentLocation` _widgetinteractor) (`SceneComponent.K2_GetComponentLocation` (`self.FlipPivot`)))) 15.0))
            (`|ExecutionSequence`
              (:`then_0`
                (`/Engine/EditorBlueprintResources/StandardMacros.DoOnce` false :!label _label_4
                  (:`Completed`
                    (set `self.InitialPageFlipPosition` (`SceneComponent.K2_GetComponentLocation` (`self.WidgetInteractor`)))
                    (set `self.InitialPageFlipTime` (`KismetSystemLibrary.GetGameTimeInSeconds`)))))
              (:`then_1`
                (goto _label_5 :!via `Reset`)))
            (else
              (`|ExecutionSequence`
                (:`then_0`
                  (goto _label_4 :!via `Reset`))
                (:`then_1`
                  (`/Engine/EditorBlueprintResources/StandardMacros.DoOnce` true :!label _label_5
                    (:`Completed`
                      (`KismetSystemLibrary.PrintString` (`KismetStringLibrary.Conv_DoubleToString` _returnvalue_3) :!enabledstate Disabled)
                      ; IfCorrectSwipe
                      (if _returnvalue_4
                        (`KismetSystemLibrary.DrawDebugLine` _returnvalue_2 (+ _returnvalue_2 (* _returnvalue 50.0)) (struct :`G` 0.969207 :`B` 1.0 :`A` 1.0) 1.0 1.0 :!enabledstate Disabled)
                        (`KismetSystemLibrary.DrawDebugLine` (`self.InitialPageFlipPosition`) _returnvalue_2 (`KismetMathLibrary.SelectColor` (struct :`R` 0.046767 :`G` 1.0 :`A` 1.0) (struct :`R` 1.0 :`G` 0.062809 :`A` 1.0) _returnvalue_4) 1.0 1.0 :!enabledstate Disabled)
                        (if (and (< _angle 30.0) _bisvalid)
                          (`self.Prev`)
                          (elif (and (> _angle 150.0) _bisvalid)
                            (`self.Next`)))))))))))))
    (else
      ; Returning to origin
      (if (and (`self.bNeedsReturn`) (`KismetSystemLibrary.IsValid` (`self.Origin`)) (not (`self.bIsReturned`)))
        (set `self.bIsReturned` true)
        (set `self.ReturnBeginTransform` (`self.GetTransform`))
        (bind (_direction _returnprogress) (`Timeline|Timeline` :!via `PlayFromStart` :!label _label_6)
          (:`Update`
            (`self.K2_SetActorTransform` (`KismetMathLibrary.TLerp` (`self.ReturnBeginTransform`) (`KismetMathLibrary.MakeTransform` (.location (`SceneComponent.K2_GetComponentToWorld` (`self.Origin`))) (.rotation (`SceneComponent.K2_GetComponentToWorld` (`self.Origin`))) (`self.GetActorScale3D`)) _returnprogress)))
          (:`Finished`
            (`self.K2_AttachToComponent` (`self.Origin`) "None" "KeepWorld" "KeepWorld" "KeepWorld" false)))))))

(event `StopReturn`
  ; Returning to origin
  (goto _label_6 :!via `Stop`))

(event `EnhancedInput|/Game/VRTemplate/Input/Actions/IA_Menu_Interact_Right_Pressed`
  (params (ActionValue :type Boolean) (ElapsedSeconds :type "Float (double-precision)") (TriggeredSeconds :type "Float (double-precision)") (InputAction :type "InputAction Object Reference" :default "/Game/VRTemplate/Input/Actions/IA_Menu_Interact_Right_Pressed.IA_Menu_Interact_Right_Pressed"))
  (bind (_bgrabbed _grabbercomponent _bright) (`self.GetGrabbedBy`))
  (bind _widgetinteractor (`self.WidgetInteractor`))
  ; UI interact
  (:`Triggered`
    (if (not _bright)
      (`WidgetInteractionComponent.PressPointerKey` _widgetinteractor "LeftMouseButton")))
  (:`Canceled`
    (if (not _bright) :!label _label_7
      (`WidgetInteractionComponent.ReleasePointerKey` _widgetinteractor "LeftMouseButton")))
  (:`Completed`
    (goto _label_7)))

(event `EnhancedInput|/Game/VRTemplate/Input/Actions/IA_Menu_Interact_Left_Pressed`
  (params (ActionValue :type Boolean) (ElapsedSeconds :type "Float (double-precision)") (TriggeredSeconds :type "Float (double-precision)") (InputAction :type "InputAction Object Reference" :default "/Game/VRTemplate/Input/Actions/IA_Menu_Interact_Left_Pressed.IA_Menu_Interact_Left_Pressed"))
  (bind (_bgrabbed _grabbercomponent _bright) (`self.GetGrabbedBy`))
  (bind _widgetinteractor (`self.WidgetInteractor`))
  ; UI interact
  (:`Triggered`
    (if _bright
      (`WidgetInteractionComponent.PressPointerKey` _widgetinteractor "LeftMouseButton")))
  (:`Canceled`
    (if _bright :!label _label_8
      (`WidgetInteractionComponent.ReleasePointerKey` _widgetinteractor "LeftMouseButton")))
  (:`Completed`
    (goto _label_8)))

(fn `AddBookSectionWithOneSetup`
  (params (SectionName :type "Text (by ref)") (PanelsWidgets :type "Array of /Game/Symbolica/Core/MultiWidgetMenu/WBP_MultiPanelWidget Class Reference (by ref)"))
  (bind _bp_booksequencemanager (`self.BP_BookSequenceManager`))
  (`BlueprintMapLibrary.Map_Add` (`self.TableOfContents`) (`/Game/Symbolica/Core/MultiWidgetMenu/BPFL_MultiWidgetMenuMisc.GetPageNumberFromSetupIndex` (`/Game/Symbolica/Core/MultiWidgetMenu/BP_BookSequenceManager.GetSetupCount` _bp_booksequencemanager) (`/Game/Symbolica/Core/MultiWidgetMenu/BP_BookSequenceManager.WidgetsCount` _bp_booksequencemanager)) SectionName)
  (`/Game/Symbolica/Core/MultiWidgetMenu/BP_BookSequenceManager.AddSetupByPanels` (`self.BP_BookSequenceManager`) PanelsWidgets))

(fn `AddBookSectionWithSetupsArray`
  (params (Name :type "Text (by ref)") (Setups :type "Array of /Game/Symbolica/Core/MultiWidgetMenu/S_MultiPanelWidgetSetup Structure (by ref)"))
  (bind _bp_booksequencemanager (`self.BP_BookSequenceManager`))
  (`BlueprintMapLibrary.Map_Add` (`self.TableOfContents`) (`/Game/Symbolica/Core/MultiWidgetMenu/BPFL_MultiWidgetMenuMisc.GetPageNumberFromSetupIndex` (`/Game/Symbolica/Core/MultiWidgetMenu/BP_BookSequenceManager.GetSetupCount` _bp_booksequencemanager) (`/Game/Symbolica/Core/MultiWidgetMenu/BP_BookSequenceManager.WidgetsCount` _bp_booksequencemanager)) Name)
  (`/Game/Symbolica/Core/MultiWidgetMenu/BP_BookSequenceManager.AddWidgetSetups` (`self.BP_BookSequenceManager`) Setups))

(fn `GetGrabbedBy`
  (returns (bGrabbed :type Boolean) (GrabberComponent :type "/Game/Symbolica/Core/Grab/BP_GrabberComponent Object Reference") (bRight :type Boolean))
  (bind _outputpin (`/Game/Symbolica/Core/BPML_Utils.GetFirstValid` (`|MakeArray` (`/Game/Symbolica/Core/Grab/BP_GrabComponent.GrabberComponent` (`self.RightHandGrab`)) (`/Game/Symbolica/Core/Grab/BP_GrabComponent.GrabberComponent` (`self.LeftHandGrab`))))
    (:`Found`
      (return true _outputpin (== (`/Game/Symbolica/Core/Grab/BP_GrabComponent.GrabberComponent` (`self.RightHandGrab`)) _outputpin)))
    (:`NotFound`
      (return false null false))))

(fn `GetSectionByPageIndex`
  (params (PageIndex :type Integer))
  (returns (SectionName :type Text) (`SectionBegin Index` :type Integer))
  (locals (SectionBeginPageIndex :type Integer))
  (bind _sectionbeginpageindex (`local.SectionBeginPageIndex`))
  (bind _keys (`BlueprintMapLibrary.Map_Keys` (`self.TableOfContents`)))
  (set `local.SectionBeginPageIndex` (`|GetArrayItem` _keys))
  (for _array_element _keys
    (if (> _array_element (+ (`local.PageIndex`) 1))
      (break)
      (else
        (set `local.SectionBeginPageIndex` _array_element))))
  (return (`BlueprintMapLibrary.Map_Find` (`self.TableOfContents`) _sectionbeginpageindex) (- _sectionbeginpageindex 1)))

(fn `OffsetFlipPivot`
  (params (bRight :type Boolean) (OffsetValue :type "Float (double-precision)"))
  (bind _returnvalue (`self.GetActorRightVector`))
  (`SceneComponent.K2_SetRelativeLocation` (`self.FlipPivot`) (* (select `bool` bRight :`false` (`KismetMathLibrary.NegateVector` _returnvalue) :`true` _returnvalue) OffsetValue) false false))

(fn `OffsetInteractor`
  (`SceneComponent.K2_SetRelativeLocation` (`self.WidgetInteractor`) (`self.InitialInteractorRelativeLocation`) false false)
  (`SceneComponent.K2_AddWorldOffset` (`self.WidgetInteractor`) (* (`self.GetActorUpVector`) (`self.InteractionOffsetValue`)) false false))

(fn `UpdateControls`
  (bind (_bgrabbed _grabbercomponent _bright) (`self.GetGrabbedBy`))
  (bind _returnvalue (`GameplayStatics.GetPlayerController` 0))
  (bind _returnvalue_2 (`GameplayStatics.GetPlayerController` 0))
  (bind _widgetinteractor (`self.WidgetInteractor`))
  (`|ExecutionSequence`
    (:`then_0`
      (`/Engine/EditorBlueprintResources/StandardMacros.IsValid` _widgetinteractor
        (:`Is Valid`
          (`SceneComponent.K2_SetRelativeLocation` _widgetinteractor (`self.InitialInteractorRelativeLocation`) false false))
        (:`Is Not Valid`
          (`self.EnableInput` _returnvalue_2)
          (`EnhancedInputSubsystemInterface.AddMappingContext` (pcsubsystem `EnhancedInputLocalPlayerSubsystem` _returnvalue_2) "/Game/VRTemplate/Input/IMC_Menu.IMC_Menu" 2 (struct)))))
    (:`then_1`
      (if _bgrabbed
        (bind _asbp_vrplayer (cast `/Game/Symbolica/Core/Player/BP_VRPlayer` (`ActorComponent.GetOwner` _grabbercomponent)))
        (set `self.PointerPosition` (select `bool` _bright :`false` (`/Game/Symbolica/Core/Player/BP_VRPlayer.RightHandCastPoint` _asbp_vrplayer) :`true` (`/Game/Symbolica/Core/Player/BP_VRPlayer.LeftHandCastPoint` _asbp_vrplayer)))
        (bind _output_get (set `self.WidgetInteractor` (select `bool` _bright :`false` (`/Game/Symbolica/Core/Player/BP_VRPlayer.RightHandWidgetInteractionComponent` _asbp_vrplayer) :`true` (`/Game/Symbolica/Core/Player/BP_VRPlayer.LeftHandWidgetInteractionComponent` _asbp_vrplayer))))
        (set `self.InitialInteractorRelativeLocation` (`SceneComponent.RelativeLocation` _output_get))
        (else
          (set `self.WidgetInteractor` null)
          (set `self.PointerPosition` null)
          (`self.DisableInput` _returnvalue)
          (`EnhancedInputSubsystemInterface.RemoveMappingContext` (pcsubsystem `EnhancedInputLocalPlayerSubsystem` _returnvalue) "/Game/VRTemplate/Input/IMC_Menu.IMC_Menu" (struct)))))))

(fn `UpdatePageSequence`
  (locals (Buffer :type Integer))
  (`|ExecutionSequence`
    (:`then_0`
      (`BlueprintMapLibrary.Map_Clear` (`self.TableOfContents`))
      (`/Game/Symbolica/Core/MultiWidgetMenu/BP_BookSequenceManager.Clear` (`self.BP_BookSequenceManager`)))
    (:`then_1`
      (`self.AddBookSectionWithOneSetup` "Title page" (`|MakeArray` "/Game/Symbolica/Core/Book/Pages/WBP_MainPage.WBP_MainPage_C" "/Game/Symbolica/Core/Book/Pages/WBP_TableOfContent.WBP_TableOfContent_C" :!type "/Game/Symbolica/Core/MultiWidgetMenu/WBP_MultiPanelWidget Class Reference")))
    (:`then_2`
      (bind _outrownames (`DataTableFunctionLibrary.GetDataTableRowNames` "/Game/Symbolica/Core/Spells/DT_Symbols.DT_Symbols"))
      (bind _sequence (`/Game/Symbolica/Core/MultiWidgetMenu/BPFL_MultiWidgetMenuMisc.MakeRepetativeSection` (`KismetArrayLibrary.Array_Length` _outrownames) "/Game/Symbolica/Core/Book/Pages/WBP_SymbolPage.WBP_SymbolPage_C" "/Game/Symbolica/Core/MultiWidgetMenu/WBP_BookPage.WBP_BookPage_C" 2))
      (`self.AddBookSectionWithSetupsArray` "Symbols" _sequence))
    (:`then_3`
      (bind _outrownames_2 (`DataTableFunctionLibrary.GetDataTableRowNames` "/Game/Symbolica/Core/Spells/DT_Spells.DT_Spells"))
      (bind _sequence_2 (`/Game/Symbolica/Core/MultiWidgetMenu/BPFL_MultiWidgetMenuMisc.MakeRepetativeSection` (`KismetArrayLibrary.Array_Length` _outrownames_2) "/Game/Symbolica/Core/Book/Pages/WBP_SpellPage.WBP_SpellPage_C" "/Game/Symbolica/Core/MultiWidgetMenu/WBP_BookPage.WBP_BookPage_C" 2))
      (`self.AddBookSectionWithSetupsArray` "Spells" _sequence_2))
    (:`then_4`
      (`self.AddBookSectionWithOneSetup` "Settings" (`|MakeArray` "/Game/Symbolica/Core/Book/Pages/WBP_SettigsLeft.WBP_SettigsLeft_C" "/Game/Symbolica/Core/Book/Pages/WBP_SettigsRight.WBP_SettigsRight_C" :!type "/Game/Symbolica/Core/MultiWidgetMenu/WBP_MultiPanelWidget Class Reference"))
      (bind _aswbp_bookmarks (cast `/Game/Symbolica/Core/Book/WBP_Bookmarks` (`WidgetComponent.GetWidget` (`self.BookmarksWidget`))))
      (`/Game/Symbolica/Core/Book/WBP_Bookmarks.CreateBookmarks` _aswbp_bookmarks (`self.TableOfContents`) (`self.BP_BookSequenceManager`)))))

(fn `UserConstructionScript`)