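; BP_Test is a test harness for the CastModel symbol-recognition model, reporting results through on-screen prints.
; On BeginPlay it waits briefly, then prints whether the model is ready.
; Separate events fill Input with sine/cosine pairs or random floats, then run GetDrawnSymbol on it and print the result or error.
; Other events print model debug info and check character lookup by index in DT_Symbols.
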(event `self.ReceiveBeginPlay`
  (`KismetSystemLibrary.Delay` 1.0)
  (`KismetSystemLibrary.PrintString` (`KismetStringLibrary.Conv_BoolToString` (`CastModelComponent.IsModelReady` (`self.CastModel`)))))

(event `MakeCircleInput`
  (bind _input (`self.Input`))
  (bind _returnvalue (/ (`self.InputSize`) 2))
  (`KismetArrayLibrary.Array_Clear` (`self.Input`))
  (for _index (range 1 (+ _returnvalue 1))
    (bind _returnvalue_2 (/ (`KismetMathLibrary.Conv_IntToDouble` _index) (`KismetMathLibrary.Conv_IntToDouble` _returnvalue)))
    (`KismetArrayLibrary.Array_Add` _input (`KismetMathLibrary.DegSin` _returnvalue_2))
    (`KismetArrayLibrary.Array_Add` _input (`KismetMathLibrary.DegCos` _returnvalue_2))))

(event `MakeRandomInput`
  (`KismetArrayLibrary.Array_Clear` (`self.Input`))
  (for _ (range 1 (+ (`self.InputSize`) 1))
    (`KismetArrayLibrary.Array_Add` (`self.Input`) (`KismetMathLibrary.RandomFloat`))))

(event `RunModel`
  (bind (_error _returnvalue) (`CastModelComponent.GetDrawnSymbol` (`self.CastModel`) (`self.Input`))
    (:`True`
      (`KismetSystemLibrary.PrintString` "Success")
      (`KismetSystemLibrary.PrintString` (`KismetStringLibrary.Conv_IntToString` _returnvalue)))
    (:`False`
      (`KismetSystemLibrary.PrintString` _error)
      (`KismetSystemLibrary.PrintString` "Hello"))))

(event `PrintDebugInfo`
  (`CastModelComponent.PrintDebugInfo` (`self.CastModel`)))

(event `CheckCharLookup`
  (bind _out_row (`/Game/Symbolica/Core/BPML_Utils.GetDataTableRowByIndex` "/Game/Symbolica/Core/Spells/DT_Symbols.DT_Symbols" (`self.Char`) true)
    (:`Row Found`
      (`KismetSystemLibrary.PrintString` (`.char_2_DECA643B49DE6BF64C353AA68062095F` (break `/Game/Symbolica/Core/Spells/S_Symbol` _out_row))))))

(fn `UserConstructionScript`)