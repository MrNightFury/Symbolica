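; VR spellcasting component that turns drawn gestures into symbols and spawns spells from symbol combinations.
; Drawn points form a spline, which is resampled at even spacing and projected onto a best-fit plane for the owner's CastModelComponent to classify.
; Recognized symbols accumulate until they match a DT_Spells row, and the spawned spell receives forwarded grab, drop and trigger input.
; SavingMode writes raw and projected points to files instead of casting.
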(event Custom|AddPoint
  (params (Position :type Vector))
  ;[0.15 0.15 0.15 0.5] Casting progress
  (Spline|AddSplinePoint (Variables|Default|GetSpline) Position "Local" true)
  (Default|SetTargetPoint (Variables|Default|GetVizualizer) Position)
  (if (Variables|Default|GetbDebugEnabled)
    (bind _returnvalue (Game|SpawnActorfromClass "/Game/Symbolica/Core/Player/BP_TestPointClass.BP_TestPointClass_C" (Math|Transform|MakeTransform Position) "Undefined" "MultiplyWithRoot" 0 2e+01 0))
    (Utilities|Array|Add (Variables|Default|GetPreview) _returnvalue)))

(event Custom|EndCast
  (bind _player (Variables|Default|GetPlayer))
  (bind _spline (Variables|Default|GetSpline))
  (bind _preview (Variables|Default|GetPreview))
  (Utilities|FlowControl|Sequence
    (:then_0
      ;[0.15 0.15 0.15 0.5] Getting fixed spaced points
      (Utilities|Array|Clear (Variables|Default|GetPoints))
      (for _index (range 0 100)
        (Utilities|Array|Add (Variables|Default|GetPoints) (Spline|GetLocationatDistanceAlongSpline _spline (|((length/100)*index) (Spline|GetSplineLength _spline) (Math|Conversions|ToFloat(Integer) _index)) "Local"))
        (if (Variables|Default|GetbDebugEnabled)
          (Rendering|Debug|DrawDebugPoint (Spline|GetLocationatDistanceAlongSpline _spline (|((length/100)*index) (Spline|GetSplineLength _spline) (Math|Conversions|ToFloat(Integer) _index)) "Local") 1e+01 "(R=1.000000,G=0.008451,B=0.000000,A=1.000000)" 2.0)))
      (Spline|ClearSplinePoints (Variables|Default|GetSpline) true))
    (:then_1
      ;[0.15 0.15 0.15 0.5] Projecting points on plane
      (bind (_d _centroid _returnvalue) (Class|Utils|GetBestFitPlane (Variables|Default|GetPoints)))
      (bind (_projectedpoints _planeorigin _returnvalue_2) (Class|Utils|ProjectPointstoPlane _returnvalue _d (Variables|Default|GetPoints) (Default|GetCameraRightVector (Variables|Default|GetPlayer)) _centroid))
      (if (Variables|Default|GetbDebugEnabled)
        (Game|SpawnActorfromClass "/Game/Symbolica/Core/Player/BP_TestPlane.BP_TestPlane_C" (Math|Transform|MakeTransform _planeorigin (Math|Conversions|RotationFromXVector _returnvalue)) "Undefined" "MultiplyWithRoot" 0 2.0 0)
        (CallFunction|DrawDebugPointsArray _projectedpoints 1e+01 "(R=0.037717,G=1.000000,B=0.000000,A=1.000000)" 2.0)))
    (:then_2
      ;[0.15 0.15 0.15 0.5] Actual casting
      (if (not (Variables|Default|GetbSavingMode))
        (bind _returnvalue_3 (Class|CastModelComponent|GetDrawnSymbol (Variables|Default|GetModelComponent) _returnvalue_2)
          (:True
            (bind _out_row (Utilities|GetDataTableRowbyIndex "/Game/Symbolica/Core/Spells/DT_Symbols.DT_Symbols" _returnvalue_3 true)
              (:Row%20Found
                (CallFunction|AddSymbol _out_row))
              (:RowNotFound
                (Utilities|IsValid _player
                  (:Is%20Valid
                    (Rendering|Components|TextRender|SetText (Variables|/Game/Symbolica/Core/Player/BP_VRPlayer.BP_VRPlayer_C|GetTextRight _player) (Utilities|Text|MakeLiteralText "404")))
                  (:Is%20Not%20Valid
                    _))))
            ;[1 0.8551 0 0.5] Clear debug preview
            (if (Variables|Default|GetbDebugEnabled) :!label _label
              (for _array_element _preview
                (Utilities|IsValid _array_element
                  (:Is%20Valid
                    (Actor|DestroyActor _array_element))))
              (Utilities|Array|Clear _preview))))))
    (:then_3
      ;[0.15 0.15 0.15 0.5] Saving points to files
      (if (Variables|Default|GetbSavingMode)
        (bind _returnvalue_4 (Math|Random|RandomInteger (Class|Utils|GetMaxInt)))
        (bind _string (CallFunction|JoinPointsArraytoString (Variables|Default|GetPoints)))
        (Class|FileHelper|WritetoFile (Utilities|String|ToString(Text) (Utilities|Text|FormatText "{id}_raw" _returnvalue_4)) _string)
        (bind _string_2 (CallFunction|Join2DPointsArraytoString _returnvalue_2))
        (Class|FileHelper|WritetoFile (Utilities|String|ToString(Text) (Utilities|Text|FormatText "{id}" _returnvalue_4)) _string_2)
        (goto _label)))))

(event Custom|AddSymbol
  (params (Symbol :type S%20Symbol%20Structure))
  (bind _vizualizer (Variables|Default|GetVizualizer))
  (bind _vizualizer_2 (Variables|Default|GetVizualizer))
  ;[0.15 0.15 0.15 0.5] Add symbol
  (Default|StopCasting _vizualizer)
  (Utilities|Array|Add (Variables|Default|GetSymbols) (.char (Utilities|Struct|BreakS_Symbol Symbol)))
  (Default|SetSymbolsDisplay _vizualizer (Variables|Default|GetSymbols))
  (bind _out_row (Utilities|ForEach "/Game/Symbolica/Core/Spells/DT_Spells.DT_Spells")
    (:LoopBody
      (if (Utilities|Array|Identical (.SymbolCombination (Utilities|Struct|BreakS_Spell _out_row)) (Variables|Default|GetSymbols))
        (bind _returnvalue (Game|SpawnActorfromClass (.Class (Utilities|Struct|BreakS_Spell _out_row)) (Transformation|GetWorldTransform) "Undefined" "MultiplyWithRoot" 0 self 0))
        (Utilities|Array|Clear (Variables|Default|GetSymbols))
        (Variables|Default|SetCurrentSpell _returnvalue)
        (Default|SetColor _vizualizer_2 (.Color (Utilities|Struct|BreakS_Spell _out_row)))
        (Default|EnableSpellCharge _vizualizer_2 true)))
    (:Completed
      ;;[0 0.609 1] TODO: Failed cast effect
      (if (>= (Utilities|Array|Length (Variables|Default|GetSymbols)) (Variables|Default|GetMaxSymbolCount))
        (Utilities|Array|Clear (Variables|Default|GetSymbols))
        (Default|SetSymbolsDisplay (Variables|Default|GetVizualizer) (Variables|Default|GetSymbols))))))

(event Custom|UpdateDisplay
  (bind _player (Variables|Default|GetPlayer))
  ;[0 0.609 1] TODO: Unified display method
  ;;[0.15 0.15 0.15 0.5] Update display
  (Utilities|IsValid _player
    (:Is%20Valid
      (Rendering|Components|TextRender|SetText (Variables|/Game/Symbolica/Core/Player/BP_VRPlayer.BP_VRPlayer_C|GetTextRight _player) (Utilities|Text|ToText(String) (Utilities|String|JoinStringArray (Variables|Default|GetSymbols) ""))))))

(event Custom|ResetSpell
  (bind _vizualizer (Variables|Default|GetVizualizer))
  ;[0.15 0.15 0.15 0.5] Spell reset
  (Utilities|FlowControl|Sequence
    (:then_0
      (Utilities|IsValid (Variables|Default|GetCurrentSpell)
        (:Is%20Valid
          (Actor|DestroyActor (Variables|Default|GetCurrentSpell))
          (Variables|Default|SetCurrentSpell 0)
          (Utilities|Array|Clear (Variables|Default|GetSymbols)))))
    (:then_1
      (Default|SetSymbolsDisplay _vizualizer (Variables|Default|GetSymbols))
      (Default|SetColor _vizualizer (Variables|Default|GetDefaultColor))
      (Default|EnableSpellCharge _vizualizer false))))

(event EventBeginPlay
  (bind _returnvalue (Components|GetOwner))
  (bind _returnvalue_2 (Actor|GetComponentbyClass _returnvalue "/Script/Symbolica.CastModelComponent"))
  ;[0.15 0.15 0.15 0.5] Get model component from owner
  (Utilities|IsValid _returnvalue_2
    (:Is%20Valid
      (Variables|Default|SetModelComponent _returnvalue_2)
      ;[0.15 0.15 0.15 0.5] Setup spline
      (bind _returnvalue_3 (Game|AddComponentbyClass _returnvalue "/Script/Engine.SplineComponent" false (Transformation|GetWorldTransform)))
      (bind _output_get (Variables|Default|SetSpline _returnvalue_3))
      (Spline|ClearSplinePoints _output_get true)
      (Class|FileHelper|EnsureBasePath)
      (bind _asbp_vrplayer (Utilities|Casting|CastToBP_VRPlayer (Components|GetOwner)))
      (Variables|Default|SetPlayer _asbp_vrplayer))
    (:Is%20Not%20Valid
      (Development|PrintString "CAST COMPONENT CANT FIND MODEL COMPONENT" true true "(R=1.000000,G=0.000000,B=0.011263,A=1.000000)" 1e+01))))

(fn PassGrabNeeded
  (bind _currentspell (Variables|Default|GetCurrentSpell))
  (Utilities|IsValid _currentspell
    (:Is%20Valid
      (return (Variables|/Game/Symbolica/Core/Spells/BP_BaseSpell.BP_BaseSpell_C|GetbPassGrab _currentspell)))
    (:Is%20Not%20Valid
      (return false))))

(fn PassDropNeeded
  (bind _currentspell (Variables|Default|GetCurrentSpell))
  (Utilities|IsValid _currentspell
    (:Is%20Valid
      (return (Variables|/Game/Symbolica/Core/Spells/BP_BaseSpell.BP_BaseSpell_C|GetbPassDrop _currentspell)))
    (:Is%20Not%20Valid
      (return false))))

(fn PassTriggerNeeded
  (bind _currentspell (Variables|Default|GetCurrentSpell))
  (Utilities|IsValid _currentspell
    (:Is%20Valid
      (return (Variables|/Game/Symbolica/Core/Spells/BP_BaseSpell.BP_BaseSpell_C|GetbPassTrigger _currentspell)))
    (:Is%20Not%20Valid
      (return false))))

(fn ClearSpell
  (Variables|Default|SetCurrentSpell 0))

(fn PassGrab
  (bind _currentspell (Variables|Default|GetCurrentSpell))
  (Utilities|IsValid _currentspell
    (:Is%20Valid
      (Default|OnGrab _currentspell))))

(fn PassDrop
  (bind _currentspell (Variables|Default|GetCurrentSpell))
  (Utilities|IsValid _currentspell
    (:Is%20Valid
      (Default|OnDrop _currentspell))))

(fn PassTrigger
  (params (Value :type Float%20%28double-precision%29))
  (bind _currentspell (Variables|Default|GetCurrentSpell))
  (Utilities|IsValid _currentspell
    (:Is%20Valid
      (Default|OnTrigger _currentspell Value))))

(fn GetSecondaryDirection
  (return (Math|Vector|RotateVector (Variables|Default|GetSecondaryDirection) (Transformation|GetWorldRotation))))