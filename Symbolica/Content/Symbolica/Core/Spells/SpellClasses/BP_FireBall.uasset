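; Grabbable fireball spell that the player throws and that explodes on impact.
; While held, Tick smooths frame-to-frame movement into a throw direction; on drop the sphere launches along it at a fixed speed and the caster's charge visual resets.
; After release, a hit beyond a safe radius from the caster's owner stops the sphere, spawns a Niagara explosion and destroys the actor after a short delay.
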(event `self.ReceiveBeginPlay`
  (`parent.ReceiveBeginPlay`)
  (set `self.LastLocation` (`self.K2_GetActorLocation`)))

(event `self.BP_GrabComponent.OnGrabbed`)

(event `self.BP_GrabComponent.OnDropped`
  (bind _caster (`self.Caster`))
  (bind _vizualizer (`/Game/Symbolica/Core/Spells/BP_CastComponent.Vizualizer` _caster))
  (bind _output_get (set `self.Speed` (* (`KismetMathLibrary.Normal` (`self.Speed`)) (`self.DefaultSpeed`))))
  (`PrimitiveComponent.SetPhysicsLinearVelocity` (`self.Sphere`) _output_get false "None")
  (`/Game/Symbolica/SpellEffects/BPI_CastVizualizer.SetColor` _vizualizer (`/Game/Symbolica/Core/Spells/BP_CastComponent.DefaultColor` _caster))
  (`/Game/Symbolica/SpellEffects/BPI_CastVizualizer.EnableSpellCharge` _vizualizer false))

(event `self.ReceiveTick`
  (params (DeltaSeconds :type "Float (single-precision)"))
  (`parent.ReceiveTick` DeltaSeconds)
  (if (`/Game/Symbolica/Core/Grab/BP_GrabComponent.bIsHeld` (`self.BP_GrabComponent`))
    (set `self.Speed` (/ (+ (- (`self.K2_GetActorLocation`) (`self.LastLocation`)) (* (`self.Speed`) (`self.SpeedCalcInertion`))) (+ (`self.SpeedCalcInertion`) 1.0)))
    (set `self.LastLocation` (`self.K2_GetActorLocation`))))

(event `EnhancedInput|/Game/Symbolica/Core/Input/IA_Walk`
  (params (ActionValue :type "Vector2D Structure") (ElapsedSeconds :type "Float (double-precision)") (TriggeredSeconds :type "Float (double-precision)") (InputAction :type "InputAction Object Reference" :default "/Game/Symbolica/Core/Input/IA_Walk.IA_Walk"))
  (:`Triggered`
    (`KismetSystemLibrary.PrintString` "Hello")))

(event `self.Sphere.OnComponentHit`
  (params (HitComponent :type "PrimitiveComponent Object Reference") (OtherActor :type "Actor Object Reference") (OtherComp :type "PrimitiveComponent Object Reference") (NormalImpulse :type "Vector Structure") (Hit :type "HitResult Structure (by ref)"))
  (if (and (and (not (`/Game/Symbolica/Core/Grab/BP_GrabComponent.bIsHeld` (`self.BP_GrabComponent`))) (`self.bIsGrabbed`)) (> (`KismetMathLibrary.Vector_Distance` (`self.K2_GetActorLocation` (`ActorComponent.GetOwner` (`self.Caster`))) (`self.K2_GetActorLocation`)) (`self.SafeExplosionRadius`)))
    (`ActorComponent.Deactivate` (`self.Niagara`))
    (`NiagaraFunctionLibrary.SpawnSystemAtLocation` "/Game/Symbolica/SpellEffects/Spells/Fireball/NS_FireballExplosion.NS_FireballExplosion" (`self.K2_GetActorLocation`) (struct) (`self.GetActorScale3D`))
    (`PrimitiveComponent.SetPhysicsLinearVelocity` (`self.Sphere`) (0.0 0.0 0.0) false "None")
    (`KismetSystemLibrary.Delay` 0.5)
    (`self.K2_DestroyActor`)))

(event `Test`
  (`NiagaraFunctionLibrary.SpawnSystemAtLocation` "/Game/Symbolica/SpellEffects/Spells/Fireball/NS_FireballExplosion.NS_FireballExplosion" (`self.K2_GetActorLocation`) (struct) (`self.GetActorScale3D`)))

(fn `UserConstructionScript`
  (`parent.UserConstructionScript`)
  (`self.SetPasses` false))