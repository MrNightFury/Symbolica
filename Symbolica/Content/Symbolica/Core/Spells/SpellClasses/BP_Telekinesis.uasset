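; Telekinesis spell that lets the caster grab objects at range with a ghost hand and pull them in.
; While free, it cone-traces forward for the best-aligned compatible grab component, moves the hand origin there and highlights it with an effect.
; Grabbing fades in the hand and enables spring-arm lag.
; Trigger input draws the object toward the spell, handing it to the caster's own grabber once within reach.
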(event `self.ReceiveBeginPlay`
  (bind _caster (`self.Caster`))
  (`/Engine/EditorBlueprintResources/StandardMacros.IsValid` _caster
    (:`Is Valid`
      (bind _grabber (message `/Game/Symbolica/Core/Grab/BPI_CanGrab.GetGrabber` (`ActorComponent.GetOwner` _caster) (`/Game/Symbolica/Core/Spells/BP_CastComponent.Type` _caster)))
      (set `self.CastersGrabber` _grabber)
      (bind _returnvalue (`PrimitiveComponent.CreateDynamicMaterialInstance` (`self.SkeletalMesh`) 0 "/Game/Symbolica/SpellEffects/Spells/MI_GhostHand.MI_GhostHand" "None"))
      (set `self.HandMaterialInstance` _returnvalue)
      (`self.ParentToCaster`))))

(event `self.ReceiveTick`
  (params (DeltaSeconds :type "Float (single-precision)"))
  (bind _selecteffect (`self.SelectEffect`))
  (if (`self.NeedsToTrace`)
    (bind (_actor _grabcomponent) (`self.Trace`))
    ; ObjectFound
    (`/Engine/EditorBlueprintResources/StandardMacros.IsValid` _grabcomponent
      (:`Is Valid`
        (bind _returnvalue (* (`/Game/Symbolica/Core/Grab/BP_GrabComponent.GrabRadius` _grabcomponent) (`Utils.GetAverageCoord` (`SceneComponent.K2_GetComponentScale` _grabcomponent))))
        (`SceneComponent.K2_SetWorldLocation` (`self.HandOrigin`) (+ (`SceneComponent.K2_GetComponentLocation` _grabcomponent) (* (`SceneComponent.GetUpVector` (`self.HandOrigin`)) _returnvalue 0.9)) false false)
        (`SceneComponent.K2_SetWorldLocation` _selecteffect (`self.K2_GetActorLocation` _actor) false false)
        (`ActorComponent.Activate` _selecteffect false)
        (`NiagaraComponent.SetVariableFloat` _selecteffect "GrabbableRadius" _returnvalue))
      (:`Is Not Valid`
        (`ActorComponent.Deactivate` (`self.SelectEffect`))))))

(event `self.OnGrab`
  (bind _bp_grabbercomponent (`self.BP_GrabberComponent`))
  (bind _returnvalue (`/Game/Symbolica/Core/Grab/BP_GrabberComponent.IsHolding` _bp_grabbercomponent))
  (`parent.OnGrab`)
  (`/Game/Symbolica/Core/Grab/BP_GrabberComponent.GrabNearComponent` _bp_grabbercomponent)
  (set `SpringArmComponent.bEnableCameraLag` _returnvalue (`self.SpringArm`))
  (`SceneComponent.SetVisibility` (`self.SkeletalMesh`) _returnvalue true)
  (bind (_direction _scale) (`Timeline|Opacity` :!label _label)
    (:`Update`
      (`MaterialInstanceDynamic.SetScalarParameterValue` (`self.HandMaterialInstance`) "Opacity" _scale))))

(event `self.OnDrop`
  (bind _bp_grabbercomponent (`self.BP_GrabberComponent`))
  (bind _returnvalue (`/Game/Symbolica/Core/Grab/BP_GrabberComponent.IsHolding` _bp_grabbercomponent))
  (`parent.OnDrop`)
  (`/Game/Symbolica/Core/Grab/BP_GrabberComponent.Release` _bp_grabbercomponent)
  (set `SpringArmComponent.bEnableCameraLag` _returnvalue (`self.SpringArm`))
  (`SceneComponent.SetVisibility` (`self.SkeletalMesh`) _returnvalue true)
  (goto _label :!via `Reverse`))

(event `self.OnTrigger`
  (params (Value :type "Float (double-precision)"))
  (bind _castersgrabber (`self.CastersGrabber`))
  (bind _returnvalue (- (`self.K2_GetActorLocation`) (`SceneComponent.K2_GetComponentLocation` (`self.HandOrigin`))))
  (`parent.OnTrigger` Value)
  (`/Engine/EditorBlueprintResources/StandardMacros.IsValid` (`/Game/Symbolica/Core/Grab/BP_GrabberComponent.GrabbedComponent` (`self.BP_GrabberComponent`))
    (:`Is Valid`
      (`|ExecutionSequence`
        (:`then_0`
          ; Move towards hand
          (`SceneComponent.K2_AddWorldOffset` (`self.HandOrigin`) (* (`KismetMathLibrary.Normal` _returnvalue) Value (`GameplayStatics.GetWorldDeltaSeconds`) (`self.MoveSpeed`)) false false)
          (`SceneComponent.K2_SetWorldLocation` (`self.SelectEffect`) (`SceneComponent.K2_GetComponentLocation` (`/Game/Symbolica/Core/Grab/BP_GrabberComponent.GrabbedComponent` (`self.BP_GrabberComponent`))) false false))
        (:`then_1`
          ; Grab if posible
          (`/Engine/EditorBlueprintResources/StandardMacros.IsValid` _castersgrabber
            (:`Is Valid`
              (bind _nearestcomponent (`/Game/Symbolica/Core/Grab/BP_GrabberComponent.GetGrabComponentNear` _castersgrabber))
              (if (and (== _nearestcomponent (`/Game/Symbolica/Core/Grab/BP_GrabberComponent.GrabbedComponent` (`self.BP_GrabberComponent`))) (< (`KismetMathLibrary.VSize` _returnvalue) (`self.GrabTolerance`)))
                (`self.OnDrop`)
                (`/Game/Symbolica/Core/Grab/BP_GrabberComponent.GrabNearComponent` _castersgrabber)))))))))

(fn `NeedsToTrace`
  (returns (ReturnValue :type Boolean))
  (bind _castersgrabber (`self.CastersGrabber`))
  (bind _returnvalue (`/Game/Symbolica/Core/Grab/BP_GrabberComponent.IsFree` (`self.BP_GrabberComponent`)))
  (`/Engine/EditorBlueprintResources/StandardMacros.IsValid` _castersgrabber
    (:`Is Valid`
      (return (and (`/Game/Symbolica/Core/Grab/BP_GrabberComponent.IsFree` _castersgrabber) _returnvalue)))
    (:`Is Not Valid`
      (return _returnvalue))))

(fn `NewFunction`)

(fn `Trace`
  (returns (Actor :type "Actor Object Reference") (GrabComponent :type "/Game/Symbolica/Core/Grab/BP_GrabComponent Object Reference"))
  (locals (CurMaxDot :type "Float (double-precision)" :default 0.0) (OptimalActor :type "Actor Object Reference") (OptimalGrabComponent :type "/Game/Symbolica/Core/Grab/BP_GrabComponent Object Reference"))
  (bind _returnvalue (`Utils.TraceCone` (`self.K2_GetActorLocation`) (`self.GetActorForwardVector`) 15.0 1000.0 20 (`|MakeArray` "ObjectTypeQuery2" "ObjectTypeQuery4" :!type "EObjectTypeQuery Enum")))
  (for _array_element _returnvalue
    (bind (_bblockinghit _binitialoverlap _time _distance _location _impactpoint _normal _impactnormal _physmat _hitactor) (`GameplayStatics.BreakHitResult` _array_element))
    (for _array_element_2 (`self.K2_GetComponentsByClass` _hitactor "/Game/Symbolica/Core/Grab/BP_GrabComponent.BP_GrabComponent_C")
      (bind _returnvalue_2 (`KismetMathLibrary.Dot_VectorVector` (`KismetMathLibrary.Normal` (- (`SceneComponent.K2_GetComponentLocation` _array_element_2) (`self.K2_GetActorLocation`))) (`self.GetActorForwardVector`)))
      (if (and (`/Game/Symbolica/Core/Grab/BP_GrabComponent.CanBeGrabbedBy` _array_element_2 (`/Game/Symbolica/Core/Grab/BP_GrabberComponent.GrabberType` (`self.BP_GrabberComponent`))) (> _returnvalue_2 (`local.CurMaxDot`)))
        (set `local.CurMaxDot` _returnvalue_2)
        (set `local.OptimalActor` _hitactor)
        (set `local.OptimalGrabComponent` _array_element_2))))
  (return (`local.OptimalActor`) (`local.OptimalGrabComponent`)))

(fn `UserConstructionScript`
  (`parent.UserConstructionScript`)
  (`self.SetPasses` true true true))