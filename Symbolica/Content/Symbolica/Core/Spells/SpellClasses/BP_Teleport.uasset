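; Teleport spell that moves the caster's owner to an aimed spot on the navmesh, targeted while grab is held and triggered on drop.
; It follows the Caster's transform and, while its secondary direction points sufficiently upward, predicts a projectile arc against static world geometry.
; The arc feeds a Niagara trail, and its hit is projected onto the navmesh to validate and place the destination sphere and mark.
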(event `self.ReceiveBeginPlay`
  (`parent.ReceiveBeginPlay`)
  (`ActorComponent.Deactivate` (`self.NS_TeleportMark`)))

(event `self.OnGrab`
  (`parent.OnGrab`)
  (set `self.IsTargeting` true)
  (`self.StartTrace`))

(event `self.OnDrop`
  (`parent.OnDrop`)
  (set `self.IsTargeting` false)
  (if (`self.bTraceSucceded`)
    (`self.TryTeleport`)))

(event `self.ReceiveTick`
  (params (DeltaSeconds :type "Float (single-precision)"))
  (bind _caster (`self.Caster`))
  (`|ExecutionSequence`
    (:`then_0`
      (`/Engine/EditorBlueprintResources/StandardMacros.IsValid` _caster
        (:`Is Valid`
          (`self.K2_SetActorTransform` (`SceneComponent.K2_GetComponentToWorld` _caster)))))
    (:`then_1`
      (if (and (`self.IsTargeting`) (> (`KismetMathLibrary.Dot_VectorVector` (`/Game/Symbolica/Core/Spells/BP_CastComponent.GetSecondaryDirection` (`self.Caster`)) (0.0 0.0 1.0)) 0.25))
        (`self.TraceUpdate` (`self.K2_GetActorLocation`) (`self.GetActorForwardVector`))
        (else
          (set `self.bTraceSucceded` false)
          (`SceneComponent.SetVisibility` (`self.Sphere1`) false false)
          (`ActorComponent.Deactivate` (`self.NS_TeleportMark`)))))))

(fn `ProjectToNavMesh`
  (params (Position :type "Vector Structure"))
  (returns (ProjectedPosition :type "Vector Structure") (IsValid :type Boolean))
  (bind (_projectedlocation _returnvalue) (`NavigationSystemV1.K2_ProjectPointToNavigation` Position null null (`self.ProjectionQueryExtent`)))
  (return _projectedlocation _returnvalue))

(fn `StartTrace`
  (`SceneComponent.SetVisibility` (`self.NS_TeleportTrace`) true false))

(fn `StopTrace`)

(fn `TraceUpdate`
  (params (StartPosition :type "Vector Structure") (ForwardVector :type "Vector Structure"))
  (bind _ns_teleportmark (`self.NS_TeleportMark`))
  (`|ExecutionSequence`
    (:`then_0`
      (bind (_outhit _outpathpositions) (`GameplayStatics.Blueprint_PredictProjectilePath_ByObjectType` StartPosition (* ForwardVector (`self.StartTraceVelocity`)) true (`self.TraceProjectileRadius`) (`|MakeArray` "ObjectTypeQuery1" :!type "EObjectTypeQuery Enum") false (`|MakeArray` null :!type "Actor Object Reference")))
      (bind _output_get (set `self.TracedPositions` _outpathpositions))
      (`KismetArrayLibrary.Array_Insert` _output_get (`local.StartPosition`))
      (bind (_projectedposition _isvalid) (`self.ProjectToNavMesh` (`.Location` (`GameplayStatics.BreakHitResult` _outhit))))
      (set `self.TraceResult` (`KismetMathLibrary.MakeVector` (.x _projectedposition) (.y _projectedposition) (- (.z _projectedposition) (`self.NavCellHeight`))))
      (if (!= (`self.bTraceSucceded`) _isvalid)
        (bind _output_get_2 (set `self.bTraceSucceded` _isvalid))
        (`SceneComponent.SetVisibility` (`self.Sphere1`) _output_get_2 false)
        (if _output_get_2
          (`ActorComponent.Activate` _ns_teleportmark false)
          (else
            (`ActorComponent.Deactivate` _ns_teleportmark)))))
    (:`then_1`
      (`NiagaraDataInterfaceArrayFunctionLibrary.SetNiagaraArrayVector` (`self.NS_TeleportTrace`) "User.PointArray" (`self.TracedPositions`))
      (`SceneComponent.K2_SetWorldLocation` (`self.Sphere1`) (`self.TraceResult`) false false)
      (`SceneComponent.K2_SetWorldLocationAndRotation` :`self` (`self.NS_TeleportMark`) :`NewLocation` (`self.TraceResult`)))))

(fn `TryTeleport`
  (bind _caster (`self.Caster`))
  (bind _returnvalue (`ActorComponent.GetOwner` _caster))
  (`self.K2_TeleportTo` _returnvalue (+ (`self.TraceResult`) (`/Game/Symbolica/Core/Spells/BP_CastComponent.GroundActorOffset` _caster)) (`self.K2_GetActorRotation` _returnvalue))
  (set `self.bTraceSucceded` false))

(fn `UserConstructionScript`
  (`parent.UserConstructionScript`)
  (`self.SetPasses` true true))