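; Manager for a multi-panel widget menu that swaps which widget each registered WidgetComponent displays.
; AddPanel registers components by name and index, and OpenMenu or OpenMenuFromArray fills those panels from a name-keyed map or an ordered array of widget classes.
; SetWidget creates each widget and passes it the manager through OnManagerInit, or clears the component for invalid classes.
; TransmitInteraction rebroadcasts interactions through OnInteraction, and failed panel lookups print debug errors.
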(event `SetWidget`
  (params (NewWidgetClass :type "/Game/Symbolica/Core/MultiWidgetMenu/WBP_MultiPanelWidget Class Reference") (WidgetComponent :type "WidgetComponent Object Reference"))
  (if (`KismetSystemLibrary.IsValidClass` NewWidgetClass)
    (bind _returnvalue (`|CreateWidget` NewWidgetClass))
    (`WidgetComponent.SetWidget` WidgetComponent _returnvalue)
    (`/Game/Symbolica/Core/MultiWidgetMenu/WBP_MultiPanelWidget.OnManagerInit` _returnvalue self)
    (else
      (`WidgetComponent.SetWidget` WidgetComponent null))))

(event `ChangeOneWidget`
  (params (PanelName :type String) (Widget :type "/Game/Symbolica/Core/MultiWidgetMenu/WBP_MultiPanelWidget Class Reference"))
  (bind _widget (`self.GetWidgetByName` PanelName)
    (:`Found`
      (`self.SetWidget` Widget _widget))))

(event `OpenMenu`
  (params (Widgets :type "Map of String to /Game/Symbolica/Core/MultiWidgetMenu/WBP_MultiPanelWidget Class Reference"))
  (bind _keys (`BlueprintMapLibrary.Map_Keys` Widgets))
  (for _array_element _keys
    (`self.ChangeOneWidget` _array_element (`BlueprintMapLibrary.Map_Find` Widgets _array_element))))

(event `OpenMenuFromArray`
  (params (Widgets :type "Array of /Game/Symbolica/Core/MultiWidgetMenu/WBP_MultiPanelWidget Class Reference"))
  (if (<= (`KismetArrayLibrary.Array_Length` Widgets) (`BlueprintMapLibrary.Map_Length` (`self.Widgets`)))
    (for (_array_element _array_index) Widgets
      (bind _widget (`self.GetWidgetByIndex` _array_index)
        (:`Found`
          (`self.SetWidget` _array_element _widget))))))

(event `AddPanel`
  (params (Name :type String) (WidgetComponent :type "WidgetComponent Object Reference") (Index :type Integer))
  (`BlueprintMapLibrary.Map_Add` (`self.WidgetIndexes`) Name Index)
  (`BlueprintMapLibrary.Map_Add` (`self.Widgets`) Index WidgetComponent))

(event `DebugPrintIncorrectArray`
  (params (Reason :type String))
  (`KismetSystemLibrary.PrintString` (`KismetStringLibrary.Concat_StrStr` "Incorrect array passed to widgets manager: " Reason) true true (struct :`R` 1.0 :`B` 0.027029 :`A` 1.0) 10.0))

(event `TransmitInteraction`
  (params (Type :type "/Game/Symbolica/Core/MultiWidgetMenu/E_InteractionTypes Enum" :default "NewEnumerator0") (Name :type String))
  (`self.OnInteraction` Type Name))

(fn `GetPanelIndexByWidget`
  (params (Widget :type "Object Object Reference"))
  (returns (Found :type Boolean) (WidgetIndex :type Integer))
  (bind _widgets (`self.Widgets`))
  (bind _keys (`BlueprintMapLibrary.Map_Keys` _widgets))
  (for _array_element _keys
    (if (== (`WidgetComponent.GetWidget` (`BlueprintMapLibrary.Map_Find` _widgets _array_element)) Widget)
      (return true _array_element)))
  (return false 0))