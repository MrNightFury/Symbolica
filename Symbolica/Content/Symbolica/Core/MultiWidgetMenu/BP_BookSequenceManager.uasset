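; BP_BookSequenceManager holds an ordered sequence of multi-panel widget setups and tracks the current page for a book-style menu.
; Setups are replaced from a page sequence, appended in bulk or singly, built from panel widgets, or cleared.
; Next, Prev and SetPage bounds-check and move the current position, then broadcast CurrentSetupChanged with the new index and widgets, leaving display to listeners.
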(event `SetPageSequence`
  (params (PageSequence :type "/Game/Symbolica/Core/MultiWidgetMenu/S_PageSequence Structure"))
  (set `self.Setups` (`.Pages_4_9A4F3B8A4BCD81AE2EF71CB93FDF15F8` (break `/Game/Symbolica/Core/MultiWidgetMenu/S_PageSequence` PageSequence))))

(event `AddWidgetSetups`
  (params (NewSequence :type "Array of /Game/Symbolica/Core/MultiWidgetMenu/S_MultiPanelWidgetSetup Structure (by ref)"))
  (`KismetArrayLibrary.Array_Append` (`self.Setups`) NewSequence))

(event `AddSetup`
  (params (Setup :type "/Game/Symbolica/Core/MultiWidgetMenu/S_MultiPanelWidgetSetup Structure (by ref)"))
  (`KismetArrayLibrary.Array_Add` (`self.Setups`) Setup))

(event `AddSetupByPanels`
  (params (PanelsWidgets :type "Array of /Game/Symbolica/Core/MultiWidgetMenu/WBP_MultiPanelWidget Class Reference"))
  (`KismetArrayLibrary.Array_Add` (`self.Setups`) (make `/Game/Symbolica/Core/MultiWidgetMenu/S_MultiPanelWidgetSetup` PanelsWidgets)))

(fn `Clear`
  (`KismetArrayLibrary.Array_Clear` (`self.Setups`)))

(fn `GetLastpageIndex`
  (returns (Index :type Integer))
  (return (`KismetArrayLibrary.Array_LastIndex` (`self.Setups`))))

(fn `GetSetupCount`
  (returns (Count :type Integer))
  (return (`KismetArrayLibrary.Array_Length` (`self.Setups`))))

(fn `Next`
  (returns (Success :type Boolean) (NewIndex :type Integer) (NewWidgets :type "/Game/Symbolica/Core/MultiWidgetMenu/S_MultiPanelWidgetSetup Structure"))
  (bind _currentposition (`self.CurrentPosition`))
  (bind _output (`|GetArrayItem` (`self.Setups`) _currentposition))
  (bind _returnvalue (>= (`self.CurrentPosition`) (`KismetArrayLibrary.Array_LastIndex` (`self.Setups`))))
  (if (not _returnvalue)
    (`/Engine/EditorBlueprintResources/StandardMacros.IncrementInt` (`self.CurrentPosition`)
      (:`  `
        (`self.CurrentSetupChanged` _currentposition _output))))
  (return (not _returnvalue) _currentposition _output))

(fn `Prev`
  (returns (Success :type Boolean) (NewIndex :type Integer) (NewWidgets :type "/Game/Symbolica/Core/MultiWidgetMenu/S_MultiPanelWidgetSetup Structure"))
  (bind _currentposition (`self.CurrentPosition`))
  (bind _output (`|GetArrayItem` (`self.Setups`) _currentposition))
  (bind _returnvalue (> (`self.CurrentPosition`) 0))
  (if _returnvalue
    (`/Engine/EditorBlueprintResources/StandardMacros.DecrementInt` (`self.CurrentPosition`)
      (:`  `
        (`self.CurrentSetupChanged` _currentposition _output))))
  (return _returnvalue _currentposition _output))

(fn `SetPage`
  (params (Index :type Integer))
  (returns (Success :type Boolean) (NewIndex :type Integer) (NewWidgets :type "/Game/Symbolica/Core/MultiWidgetMenu/S_MultiPanelWidgetSetup Structure"))
  (bind _currentposition (`self.CurrentPosition`))
  (bind _output (`|GetArrayItem` (`self.Setups`) _currentposition))
  (bind _returnvalue (and (>= Index 0) (<= Index (`KismetArrayLibrary.Array_LastIndex` (`self.Setups`)))))
  (if _returnvalue
    (set `self.CurrentPosition` Index)
    (`self.CurrentSetupChanged` _currentposition _output))
  (return _returnvalue _currentposition _output))