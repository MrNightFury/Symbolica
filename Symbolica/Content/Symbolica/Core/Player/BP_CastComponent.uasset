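; Player cast component that turns a drawn stroke into a recognized symbol, displayed on the VR player's right text.
; AddPoint builds a runtime spline, which EndCast resamples at even spacing and projects onto a least-squares best-fit plane using the camera's right vector.
; The flattened 2D points go to the owner's CastModelComponent, whose result indexes DT_Symbols.
; SavingMode instead writes raw and projected points to files; DebugEnabled visualizes each stage.
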(event Custom|AddPoint
  (params (Position :type Vector))
  ;[0.15 0.15 0.15 0.5] Casting progress
  (Spline|AddSplinePoint (Variables|Default|GetSpline) Position "Local" true)
  (if (Variables|Default|GetbDebugEnabled)
    (bind _returnvalue (Game|SpawnActorfromClass "/Game/Symbolica/Core/Player/BP_TestPointClass.BP_TestPointClass_C" (Math|Transform|MakeTransform Position) "Undefined" "MultiplyWithRoot" 0 2e+01 0))
    (Utilities|Array|Add (Variables|Default|GetPreview) _returnvalue)))

(event Custom|EndCast
  (bind _player (Variables|Default|GetPlayer))
  (bind _spline (Variables|Default|GetSpline))
  (bind _preview (Variables|Default|GetPreview))
  (bind _textright (Variables|/Game/Symbolica/Core/Player/BP_VRPlayer1.BP_VRPlayer1_C|GetTextRight _player))
  (Utilities|FlowControl|Sequence
    (:then_0
      ;[0.15 0.15 0.15 0.5] Getting fixed spaced points
      (Utilities|Array|Clear (Variables|Default|GetPoints))
      (for _index (range 0 100)
        (Utilities|Array|Add (Variables|Default|GetPoints) (Spline|GetLocationatDistanceAlongSpline _spline (|((length/100)*index) (Spline|GetSplineLength _spline) (Math|Conversions|ToFloat(Integer) _index)) "Local"))
        (if (Variables|Default|GetbDebugEnabled)
          (Rendering|Debug|DrawDebugPoint (Spline|GetLocationatDistanceAlongSpline _spline (|((length/100)*index) (Spline|GetSplineLength _spline) (Math|Conversions|ToFloat(Integer) _index)) "Local") 1e+01 "(R=1.000000,G=0.008451,B=0.000000,A=1.000000)" 2.0)))
      (Spline|ClearSplinePoints (Variables|Default|GetSpline) true))
    (:then_1
      ;[0.15 0.15 0.15 0.5] Projecting points on plane
      (bind (_d _centroid _returnvalue) (Class|Utils|GetBestFitPlaneMinSquares (Variables|Default|GetPoints)))
      (bind (_projectedpoints _planeorigin _returnvalue_2) (Class|Utils|ProjectPointstoPlane _returnvalue _d (Variables|Default|GetPoints) (Default|GetCameraRightVector (Variables|Default|GetPlayer)) _centroid))
      (if (Variables|Default|GetbDebugEnabled)
        (Game|SpawnActorfromClass "/Game/Symbolica/Core/Player/BP_TestPlane.BP_TestPlane_C" (Math|Transform|MakeTransform _planeorigin (Math|Conversions|RotationFromXVector _returnvalue)) "Undefined" "MultiplyWithRoot" 0 2.0 0)
        (CallFunction|DrawDebugPointsArray _projectedpoints 1e+01 "(R=0.037717,G=1.000000,B=0.000000,A=1.000000)" 2.0)))
    (:then_2
      ;[0.15 0.15 0.15 0.5] Actual casting
      (if (not (Variables|Default|GetbSavingMode))
        (bind _returnvalue_3 (Class|CastModelComponent|GetDrawnSymbol (Variables|Default|GetModelComponent) (Class|Utils|Flatten2D _returnvalue_2))
          (:True
            (bind _out_row (Utilities|GetDataTableRowbyIndex "/Game/Symbolica/Core/Spells/DT_Symbols.DT_Symbols" _returnvalue_3 true)
              (:Row%20Found
                (Rendering|Components|TextRender|SetText _textright (Utilities|Text|ToText(String) (Utilities|Struct|BreakS_Symbol _out_row)))
                (if (Variables|Default|GetbDebugEnabled) :!label _label
                  (for _array_element _preview
                    (Utilities|IsValid _array_element
                      (:Is%20Valid
                        (Actor|DestroyActor _array_element))))
                  (Utilities|Array|Clear _preview)))
              (:RowNotFound
                (Rendering|Components|TextRender|SetText _textright (Utilities|Text|MakeLiteralText "Error!"))))))))
    (:then_3
      ;[0.15 0.15 0.15 0.5] Saving points to files
      (if (Variables|Default|GetbSavingMode)
        (bind _returnvalue_4 (Math|Random|RandomInteger (Class|Utils|GetMaxInt)))
        (bind _string (CallFunction|JoinPointsArraytoString (Variables|Default|GetPoints)))
        (Class|FileHelper|WritetoFile (Utilities|String|ToString(Text) (Utilities|Text|FormatText "{id}_raw" _returnvalue_4)) _string)
        (bind _string_2 (CallFunction|Join2DPointsArraytoString _returnvalue_2))
        (Class|FileHelper|WritetoFile (Utilities|String|ToString(Text) (Utilities|Text|FormatText "{id}" _returnvalue_4)) _string_2)
        (goto _label)))))

(event EventBeginPlay
  (bind _returnvalue (Components|GetOwner))
  (bind _returnvalue_2 (Actor|GetComponentbyClass _returnvalue "/Script/Symbolica.CastModelComponent"))
  ;[0.15 0.15 0.15 0.5] Get model component from owner
  (Utilities|IsValid _returnvalue_2
    (:Is%20Valid
      (Variables|Default|SetModelComponent _returnvalue_2)
      ;[0.15 0.15 0.15 0.5] Setup spline
      (bind _returnvalue_3 (Game|AddComponentbyClass _returnvalue "/Script/Engine.SplineComponent" false (Transformation|GetWorldTransform)))
      (bind _output_get (Variables|Default|SetSpline _returnvalue_3))
      (Spline|ClearSplinePoints _output_get true)
      (Class|FileHelper|EnsureBasePath)
      (bind _asbp_vrplayer_1 (Utilities|Casting|CastToBP_VRPlayer1 (Components|GetOwner)))
      (Variables|Default|SetPlayer _asbp_vrplayer_1))
    (:Is%20Not%20Valid
      (Development|PrintString "CAST COMPONENT CANT FIND MODEL COMPONENT" true true "(R=1.000000,G=0.000000,B=0.011263,A=1.000000)" 1e+01))))