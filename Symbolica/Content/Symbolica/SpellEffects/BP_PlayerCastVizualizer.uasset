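; Scene component that visualizes the player's spellcasting through an attached Niagara effect and an optional text display.
; It keeps the effect's origin on the owner each tick and exposes events for activation, color, spell charge sparks and symbol text.
; Setting a target point updates a relative offset and starts sparks.
; Stopping casting disables them and briefly pulses a combine flag over two ticks.
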(event `self.ReceiveTick`
  (params (DeltaSeconds :type "Float (single-precision)"))
  (`NiagaraComponent.SetVariablePosition` (`self.Niagara`) "Origin" (`Actor.K2_GetActorLocation` (`self.Owner`))))

(event `self.ReceiveBeginPlay`
  (bind _niagara (`self.Niagara`))
  (set `self.Owner` (`self.GetOwner`))
  (bind _returnvalue (`NiagaraFunctionLibrary.SpawnSystemAttached` "/Game/Symbolica/SpellEffects/NS_Sorcererment.NS_Sorcererment" self "None" (0.0 0.0 0.0) (struct) "KeepRelativeOffset"))
  (bind _output_get (set `self.Niagara` _returnvalue))
  (`NiagaraComponent.SetAsset` _output_get "/Game/Symbolica/SpellEffects/NS_Sorcererment.NS_Sorcererment" true)
  (`FXSystemComponent.SetEmitterEnable` _niagara "Sparks" false)
  (`FXSystemComponent.SetColorParameter` _niagara "MainColor" (struct :`R` 0.45625 :`B` 0.421216 :`A` 1.0))
  (`self.EnableSpellCharge` false))

(event `/Game/Symbolica/SpellEffects/BPI_CastVizualizer.SetEnabled`
  (params (bEnabled :type Boolean))
  (bind _niagara (`self.Niagara`))
  (if bEnabled
    (`self.Activate` _niagara false)
    (else
      (`self.Deactivate` _niagara))))

(event `/Game/Symbolica/SpellEffects/BPI_CastVizualizer.SetTargetPoint`
  (params (Point :type "Vector Structure"))
  (`NiagaraComponent.SetVariableVec3` (`self.Niagara`) "TargetOffset" (- Point (`Actor.K2_GetActorLocation` (`self.Owner`))))
  (if (not (`self.bIsCasting`))
    (`FXSystemComponent.SetEmitterEnable` (`self.Niagara`) "Sparks" true)
    (set `self.bIsCasting` true)))

(event `/Game/Symbolica/SpellEffects/BPI_CastVizualizer.StopCasting`
  (`self.Combine`)
  (`FXSystemComponent.SetEmitterEnable` (`self.Niagara`) "Sparks" false)
  (set `self.bIsCasting` false))

(event `/Game/Symbolica/SpellEffects/BPI_CastVizualizer.SetTextDisplay`
  (params (TextRenderComponent :type "TextRenderComponent Object Reference"))
  (set `self.TextDisplay` TextRenderComponent))

(event `/Game/Symbolica/SpellEffects/BPI_CastVizualizer.SetSymbolsDisplay`
  (params (Symbols :type "Array of String (by ref)"))
  (bind _textdisplay (`self.TextDisplay`))
  (`/Engine/EditorBlueprintResources/StandardMacros.IsValid` _textdisplay
    (:`Is Valid`
      (`TextRenderComponent.K2_SetText` _textdisplay (`KismetTextLibrary.Conv_StringToText` (`KismetStringLibrary.JoinStringArray` Symbols))))))

(event `/Game/Symbolica/SpellEffects/BPI_CastVizualizer.EnableSpellCharge`
  (params (Enable :type Boolean))
  (`FXSystemComponent.SetEmitterEnable` (`self.Niagara`) "SparksLocal" Enable))

(event `/Game/Symbolica/SpellEffects/BPI_CastVizualizer.SetColor`
  (params (Color :type "LinearColor Structure"))
  (`NiagaraComponent.SetVariableLinearColor` (`self.Niagara`) "MainColor" Color))

(event `/Game/Symbolica/SpellEffects/BPI_CastVizualizer.Combine`
  (`NiagaraComponent.SetVariableBool` (`self.Niagara`) "GlobalToCombine" true)
  (`KismetSystemLibrary.DelayUntilNextTick`)
  (`KismetSystemLibrary.DelayUntilNextTick`)
  (`NiagaraComponent.SetVariableBool` (`self.Niagara`) "GlobalToCombine" false))