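; BP_NSTest is a test actor for the NSPlayerCastVizualizer Niagara spell-casting effect.
; ToggleCasting flip-flops between targeting the actor's own location and stopping the cast, while Toggle flip-flops the effect's enabled state, both through message calls on the visualizer.
; The construction script also sets the target to the actor's location.
; Direct toggles of the Runes emitter are left unconnected.
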(event `ToggleCasting`
  (bind _ns_playercastvizualizer (`self.NS_PlayerCastVizualizer`))
  (`/Engine/EditorBlueprintResources/StandardMacros.FlipFlop`
    (:`A`
      (message `/Game/Symbolica/SpellEffects/BPI_CastVizualizer.SetTargetPoint` _ns_playercastvizualizer (+ (`self.K2_GetActorLocation`) (0.0 0.0 0.0))))
    (:`B`
      (message `/Game/Symbolica/SpellEffects/BPI_CastVizualizer.StopCasting` _ns_playercastvizualizer))))

(event `Toggle`
  (bind _ns_playercastvizualizer (`self.NS_PlayerCastVizualizer`))
  (`/Engine/EditorBlueprintResources/StandardMacros.FlipFlop`
    (:`A`
      (message `/Game/Symbolica/SpellEffects/BPI_CastVizualizer.SetEnabled` _ns_playercastvizualizer true))
    (:`B`
      (message `/Game/Symbolica/SpellEffects/BPI_CastVizualizer.SetEnabled` _ns_playercastvizualizer false))))

(fn `UserConstructionScript`
  (message `/Game/Symbolica/SpellEffects/BPI_CastVizualizer.SetTargetPoint` (`self.NS_PlayerCastVizualizer`) (`self.K2_GetActorLocation`)))