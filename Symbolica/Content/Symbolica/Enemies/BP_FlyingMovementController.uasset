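; Actor component that drives physics-based flying movement for its owner, apparently an enemy, through Flight, Drag and Dash states processed on Tick.
; MoveTo starts Flight, which faces the target, accelerates forward up to a speed cap and damps off-axis velocity to curb drift.
; Stop enters Drag, slowing by linear plus flat drag.
; Dash sets a timed velocity burst, then switches to Drag and signals the state change.
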(event `self.ReceiveTick`
  (params (DeltaSeconds :type "Float (single-precision)"))
  (`KismetSystemLibrary.PrintString` "Hello" true true (struct :`G` 0.66 :`B` 1.0 :`A` 1.0) 2.0 (`KismetStringLibrary.Conv_StringToName` (`KismetStringLibrary.Concat_StrStr` (`KismetSystemLibrary.GetDisplayName` self) "_Move")))
  (switch `/Game/Symbolica/Enemies/E_FlightStates` (`self.MoveState`)
    (:`NewEnumerator0`
      (`self.ProcessMove` DeltaSeconds))
    (:`NewEnumerator1`
      (`self.ProcessDrag` DeltaSeconds))
    (:`NewEnumerator2`
      (`self.ProcessDash` DeltaSeconds))))

(event `SetState`
  (params (State :type "/Game/Symbolica/Enemies/E_FlightStates Enum" :default "NewEnumerator0"))
  (set `self.MoveState` State))

(fn `CalcDrag`
  (params (Value :type "Vector Structure") (Drag :type "Float (double-precision)") (DeltaTime :type "Float (double-precision)"))
  (returns (DraggedValue :type "Vector Structure"))
  (return (* Value (- 1.0 (* Drag DeltaTime)))))

(fn `Dash`
  (params (DIrection :type "Vector Structure"))
  (bind _root (`self.GetOwnerRootComponent`))
  (`KismetSystemLibrary.PrintString` "Dash started")
  (`PrimitiveComponent.WakeRigidBody` _root "None")
  (`PrimitiveComponent.SetPhysicsLinearVelocity` _root (* DIrection (`self.DashSpeed`)) false "None")
  (set `self.MoveState` "NewEnumerator2")
  (set `self.RemainingDashTime` (`self.TimeToDash`))
  (`Actor.K2_SetActorRotation` (`self.GetOwner`) (`KismetMathLibrary.Conv_VectorToRotator` DIrection) false))

(fn `GetOwnerLocation`
  (returns (Location :type "Vector Structure"))
  (return (`Actor.K2_GetActorLocation` (`self.GetOwner`))))

(fn `GetOwnerRootComponent`
  (returns (Root :type "PrimitiveComponent Object Reference"))
  (bind _asprimitive_component (cast `PrimitiveComponent` (`Actor.RootComponent` (`self.GetOwner`)))
    (:`then`
      _)
    (:`CastFailed`
      _))
  (return _asprimitive_component))

(fn `MoveTo`
  (params (Location :type "Vector Structure"))
  (bind _root (`self.GetOwnerRootComponent`))
  (set `self.Target` Location)
  (set `self.MoveState` "NewEnumerator0")
  (`PrimitiveComponent.WakeRigidBody` _root "None")
  (`SceneComponent.K2_AddWorldOffset` _root (0.0 0.0 1.0) false false))

(fn `ProcessDash`
  (params (DeltaTime :type "Float (double-precision)"))
  (bind _output_get (set `self.RemainingDashTime` (- (`self.RemainingDashTime`) DeltaTime)))
  (if (< _output_get 0.0)
    (set `self.MoveState` "NewEnumerator1")
    (`self.MovementStateChanged` "NewEnumerator1")
    (`KismetSystemLibrary.PrintString` "Dash finished")))

(fn `ProcessDrag`
  (params (DeltaTime :type "Float (double-precision)"))
  (bind _returnvalue (`PrimitiveComponent.GetPhysicsLinearVelocity` (`self.GetOwnerRootComponent`) "None"))
  (`PrimitiveComponent.SetPhysicsLinearVelocity` (`self.GetOwnerRootComponent`) (* (`KismetMathLibrary.Normal` _returnvalue) (`KismetMathLibrary.FMax` (- (* (`KismetMathLibrary.VSize` _returnvalue) (- 1.0 (* (`self.LinearDrag`) (`local.DeltaTime`)))) (* (`self.FlatDrag`) (`local.DeltaTime`))))) false "None"))

(fn `ProcessMove`
  (params (DeltaTime :type "Float (double-precision)"))
  (locals (CurVelocity :type "Vector Structure" :default (0.0 0.0 0.0)) (CurRotation :type "Rotator Structure"))
  (bind _root (`self.GetOwnerRootComponent`))
  (bind _curvelocity (`local.CurVelocity`))
  (bind _returnvalue (`KismetMathLibrary.GetForwardVector` (`local.CurRotation`)))
  (bind _returnvalue_2 (* (`KismetMathLibrary.Dot_VectorVector` _curvelocity _returnvalue) _returnvalue))
  (bind _returnvalue_3 (+ (`self.CalcDrag` (- _curvelocity _returnvalue_2) (`self.NonRightDirectionDrag`) (`local.DeltaTime`)) (+ _returnvalue_2 (* _returnvalue (`local.DeltaTime`) (`self.Acceleration`)))))
  (bind _returnvalue_4 (* (`KismetMathLibrary.FMin` (`KismetMathLibrary.VSize` _returnvalue_3) (`self.MaxVelocity`)) (`KismetMathLibrary.Normal` _returnvalue_3)))
  (`|ExecutionSequence`
    (:`then_0`
      (bind _output_get (set `local.CurRotation` (`KismetMathLibrary.FindLookAtRotation` (`self.GetOwnerLocation`) (`self.Target`))))
      (`Actor.K2_SetActorRotation` (`self.GetOwner`) _output_get false)
      (bind _returnvalue_5 (`PrimitiveComponent.GetPhysicsLinearVelocity` _root "None"))
      (set `local.CurVelocity` _returnvalue_5)
      (`PrimitiveComponent.SetPhysicsAngularVelocityInDegrees` _root (0.0 0.0 0.0) false "None"))
    (:`then_1`
      (`PrimitiveComponent.SetPhysicsLinearVelocity` (`self.GetOwnerRootComponent`) _returnvalue_4 false "None")
      (`KismetSystemLibrary.PrintString` (`KismetStringLibrary.Conv_VectorToString` _returnvalue_4) true true (struct :`G` 0.66 :`B` 1.0 :`A` 1.0) 2.0 "T"))))

(fn `Stop`
  (set `self.MoveState` "NewEnumerator1"))