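; BP_Ghost is a flying ghost enemy with a physics collider, driven by a StateTree and a flying movement controller.
; AI perception stores actors tagged as player faction as Target and notifies the StateTree, while damage switches movement state and sends a Damaged event.
; The construction script scatters ten Niagara components at small random offsets around it.
; Debug helpers print velocity and apply an upward test impulse.
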(event `self.ReceiveTick`
  (params (DeltaSeconds :type "Float (single-precision)"))
  (bind _returnvalue (`PrimitiveComponent.GetPhysicsLinearVelocity` (`self.Collider`) "None"))
  (`KismetSystemLibrary.PrintString` (`KismetStringLibrary.Conv_DoubleToString` (`KismetMathLibrary.VSize` _returnvalue)) true true (struct :`G` 0.66 :`B` 1.0 :`A` 1.0) 2.0 "VEL"))

(event `self.ReceiveBeginPlay`
  (set `self.TargetLocation` (`self.K2_GetActorLocation` (`self.Spawn`))))

(event `self.AIPerception.OnPerceptionUpdated`
  (params (UpdatedActors :type "Array of Actor Object Reference (by ref)"))
  (for _array_element UpdatedActors
    (if (`BlueprintGameplayTagLibrary.HasTag` (`BlueprintGameplayTagLibrary.GetOwnedGameplayTags` (`BlueprintGameplayTagLibrary.Conv_ObjectToGameplayTagAssetInterface` _array_element)) (struct :`TagName` "AI.Faction.Player"))
      (set `self.Target` _array_element)
      (`StateTreeComponent.SendStateTreeEvent` (`self.StateTree`) (make `StateTreeEvent` (struct :`TagName` "AI.Events.TargetSpotted"))))))

(event `self.BP_HealthComponent.OnDamageGot`
  (params (Damage :type "Float (double-precision)") (DamageType :type "GameplayTag Structure") (DamageCauser :type "Actor Object Reference"))
  (`/Game/Symbolica/Enemies/BP_FlyingMovementController.SetState` (`self.BP_FlyingMovementController`) "NewEnumerator1")
  (`StateTreeComponent.SendStateTreeEvent` (`self.StateTree`) (make `StateTreeEvent` (struct :`TagName` "AI.Events.Damaged")))
  (`KismetSystemLibrary.PrintString` "Damaged" true true (struct :`R` 1.0 :`G` 0.712717 :`A` 1.0) 2.0 (`KismetStringLibrary.Conv_StringToName` (`KismetSystemLibrary.GetDisplayName` self))))

(event `DEBUG_AddImpulse`
  (`/Game/Symbolica/Enemies/BP_FlyingMovementController.SetState` (`self.BP_FlyingMovementController`) "NewEnumerator3")
  (`PrimitiveComponent.AddImpulse` (`self.Collider`) (* (0.0 0.0 1.0) (`self.DEBUG_Impulse`)) "None" false)
  (`StateTreeComponent.SendStateTreeEvent` (`self.StateTree`) (make `StateTreeEvent` (struct :`TagName` "AI.Events.Damaged"))))

(fn `UserConstructionScript`
  (for _ (range 1 11)
    (`AddComponent|NODE_AddNiagaraComponent-1` :`RelativeTransform` (`KismetMathLibrary.MakeTransform` (* (`KismetMathLibrary.RandomUnitVector`) 5.0)))))