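; BP_GhostSpawn is a spawn point that creates a BP_Ghost at its own transform when SpawnGhost fires, passing itself to the ghost as its Spawn reference.
; The construction script sizes the Sphere component to IdleRadius and briefly draws a debug plane to show the bottom of that volume.
; GetBottomPlane builds that plane along the actor's up axis, BottomHeight above the sphere's lowest point.
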(event `SpawnGhost`
  (`|SpawnActorFromClass` "/Game/Symbolica/Enemies/BP_Ghost.BP_Ghost_C" (`self.GetTransform`) "Undefined" "MultiplyWithRoot" null self null))

(fn `GetBottomPlane`
  (returns (Plane :type "Plane Structure"))
  (bind _returnvalue (`self.GetActorUpVector`))
  (return (`KismetMathLibrary.MakePlaneFromPointAndNormal` (+ (`self.K2_GetActorLocation`) (* (`KismetMathLibrary.NegateVector` _returnvalue) (- (`self.IdleRadius`) (`self.BottomHeight`)))) _returnvalue)))

(fn `UserConstructionScript`
  (`SphereComponent.SetSphereRadius` (`self.Sphere`) (`self.IdleRadius`) true)
  (`KismetSystemLibrary.DrawDebugPlane` (`self.GetBottomPlane`) (`self.K2_GetActorLocation`) 100.0 (struct :`R` 1.0 :`G` 1.0 :`B` 1.0 :`A` 1.0) 1.0))